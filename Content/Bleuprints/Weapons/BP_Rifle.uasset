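; Rifle weapon Blueprint that provides automatic fire for as long as shooting is active.
; StartShooting calls FFireWeapon and plays the gun mesh fire animation immediately, then starts a looping FireRate timer that repeats both through FireRifle.
; StopShooting clears and invalidates the stored timer handle to end the burst.
; The shot logic itself sits in FFireWeapon, which is not defined in these graphs.
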(event Custom|FireRifle
  (CallFunction|FFireWeapon)
  (Components|Animation|PlayAnimation (Variables|Default|GetGunMesh) "/Game/MilitaryWeapSilver/Weapons/Animations/Fire_Rifle_W.Fire_Rifle_W" false))

(event EventBeginPlay
  (|CallParentFunction) ; This node is disabled and will not be called.\nDrag off pins to build functionality.
)

(event Collision|EventActorBeginOverlap
  (params (OtherActor :type Actor%20Object%20Reference))
  (|CallParentFunction OtherActor) ; This node is disabled and will not be called.\nDrag off pins to build functionality.
)

(event EventTick
  (params (DeltaSeconds :type Float%20%28single-precision%29))
  (|CallParentFunction DeltaSeconds) ; This node is disabled and will not be called.\nDrag off pins to build functionality.
)

(event EventStartShooting
  (CallFunction|FFireWeapon)
  (Components|Animation|PlayAnimation (Variables|Default|GetGunMesh) "/Game/MilitaryWeapSilver/Weapons/Animations/Fire_Rifle_W.Fire_Rifle_W" false)
  (bind _returnvalue (Utilities|Time|SetTimerbyEvent (delegate Custom|FireRifle) (Variables|Default|GetFireRate) true))
  (Variables|Default|SetFireEvent _returnvalue))

(event EventStopShooting
  (Utilities|Time|ClearandInvalidateTimerbyHandle (Variables|Default|GetFireEvent)))

(fn ConstructionScript
  (|CallParentFunction))